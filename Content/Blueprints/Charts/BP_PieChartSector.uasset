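; Clickable 3D pie chart sector actor that switches UI panels when selected.
; On BeginPlay it builds its chart shape through Set3DPieChart using the base style, its color and a sector gap.
; A click passes its section index to SwitchPanel on top-level widgets of a class.
; Every Tick, three text renders turn toward the player pawn, with pitch clamped to a slight downward range.
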(event `self.ReceiveBeginPlay`
  (`parent.ReceiveBeginPlay`)
  (`self.Set3DPieChart` "Base" (`self.Pie Chart Color`) "SectorGap"))

(event `self.ReceiveActorOnClicked`
  (params (ButtonPressed :type "Key Structure"))
  (bind _returnvalue (`self.GetSectionIndex`))
  (bind _foundwidgets (`WidgetBlueprintLibrary.GetAllWidgetsOfClass` null))
  (for _array_element _foundwidgets
    (`self.Switch Panel` _array_element _returnvalue)))

(event `self.ReceiveTick`
  (params (DeltaSeconds :type "Float (single-precision)"))
  (`self.Update Rotation` (`self.TextRender`))
  (`self.Update Rotation` (`self.TextRender1`))
  (`self.Update Rotation` (`self.TextRender2`)))

(fn `Update Rotation`
  (params (InTextTarget :type "TextRenderComponent Object Reference"))
  (bind (_returnvalue_roll _returnvalue_pitch _returnvalue_yaw) (`KismetMathLibrary.BreakRotator` (`KismetMathLibrary.FindLookAtRotation` (`SceneComponent.K2_GetComponentLocation` InTextTarget) (`self.K2_GetActorLocation` (`GameplayStatics.GetPlayerPawn` 0)))))
  (`SceneComponent.K2_SetWorldRotation` InTextTarget (`KismetMathLibrary.MakeRotator` _returnvalue_roll (`KismetMathLibrary.FClamp` _returnvalue_pitch -10.0 0.0) _returnvalue_yaw) false false))

(fn `UserConstructionScript`
  (`parent.UserConstructionScript`))